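; BP_Checkpoint is a checkpoint actor that records a respawn point for the player and changes color once touched.
; On BeginPlay it creates a dynamic material instance on its cylinder and tints it with the start color.
; When a BP_ThirdPersonCharacter overlaps it, it passes its own transform, raised along Z, to the character's SetCheckpoint and switches the material to the checked color.
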(event `self.ReceiveBeginPlay`
  (bind _returnvalue (`PrimitiveComponent.CreateDynamicMaterialInstance` (`self.Cylinder`) 0 "/Game/BP_ProfMoto/Checkpoint/ColorShiftMaterial.ColorShiftMaterial" "None"))
  (bind _output_get (set `self.CheckpointMaterial` _returnvalue))
  (`MaterialInstanceDynamic.SetVectorParameterValue` _returnvalue "Color" (`self.StartColor`))
  (`MaterialInstanceDynamic.SetVectorParameterValue` _output_get "Color" (`self.StartColor`)))

(event `self.ReceiveActorBeginOverlap`
  (params (OtherActor :type "Actor Object Reference"))
  (bind _asbp_third_person_character (cast `/Game/ThirdPerson/Blueprints/BP_ThirdPersonCharacter` OtherActor))
  (`/Game/ThirdPerson/Blueprints/BP_ThirdPersonCharacter.SetCheckpoint` _asbp_third_person_character (`KismetMathLibrary.MakeTransform` (`KismetMathLibrary.MakeVector` (.x (.location (`self.GetTransform`))) (.y (.location (`self.GetTransform`))) (+ (.z (.location (`self.GetTransform`))) 150.0)) (.rotation (`self.GetTransform`)) (.scale (`self.GetTransform`))))
  (`MaterialInstanceDynamic.SetVectorParameterValue` (`self.CheckpointMaterial`) "Color" (`self.CheckedColor`)))

(fn `UserConstructionScript`)