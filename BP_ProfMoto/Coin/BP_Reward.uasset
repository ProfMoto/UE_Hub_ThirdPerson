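; BP_Reward is a coin-gated reward actor that appears or disappears when the coin count reaches CoinsToUnlock.
; OnAsReward picks the direction by setting visibility and collision, hiding the actor on BeginPlay if it is meant to appear.
; CoinCheck toggles it immediately and calls AutoRewardID on BP_CoinManager, or with OverlapToTrigger only flags success for ActorBeginOverlap to apply.
; ConsumeCoinsOnUse optionally deducts the cost through the manager.
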(event `CoinCheck`
  (params (CoinToCheck :type Integer))
  ; Check Coin Count against Coins Needed
  (if (>= CoinToCheck (`self.CoinsToUnlock`))
    (if (`self.OverlapToTrigger`)
      (set `self.CheckSuccess` true)
      (else
        (`SceneComponent.SetVisibility` (`self.DefaultSceneRoot`) (`self.OnAsReward`) true)
        (`self.SetActorEnableCollision` (`self.OnAsReward`))
        (`/Game/BP_ProfMoto/Coin/BP_CoinManager.AutoRewardID++` (`self.ManagerRef`))
        (if (`self.ConsumeCoinsOnUse`)
          (`self.ConsumeCoins`))))))

(event `self.ReceiveBeginPlay`
  (bind _returnvalue (`GameplayStatics.GetActorOfClass` "/Game/BP_ProfMoto/Coin/BP_CoinManager.BP_CoinManager_C"))
  (set `self.ManagerRef` _returnvalue)
  ; Turn off object on Begin if On as Reward is checked
  (if (`self.OnAsReward`)
    (`SceneComponent.SetVisibility` (`self.DefaultSceneRoot`) false true)
    (`self.SetActorEnableCollision` false)))

(event `self.ReceiveActorBeginOverlap`
  (params (OtherActor :type "Actor Object Reference"))
  ; On Overlap change Visibility/Collisions if Overlap to Trigger is checked
  (if (`self.OverlapToTrigger`)
    (bind _returnvalue (`GameplayStatics.GetActorOfClass` "/Game/BP_ProfMoto/Coin/BP_CoinManager.BP_CoinManager_C"))
    (`self.CoinCheck` (`/Game/BP_ProfMoto/Coin/BP_CoinManager.CoinCount` _returnvalue))
    (if (`self.CheckSuccess`)
      (`SceneComponent.SetVisibility` (`self.DefaultSceneRoot`) (`self.OnAsReward`) true)
      (`self.SetActorEnableCollision` (`self.OnAsReward`))
      (if (`self.ConsumeCoinsOnUse`)
        (`self.ConsumeCoins`)))))

(event `ConsumeCoins`
  ; Subtract Coins if Consume Coins on Use is checked
  (`/Game/BP_ProfMoto/Coin/BP_CoinManager.ConsumeCoins` (`self.ManagerRef`) (`self.CoinsToUnlock`)))

(fn `UserConstructionScript`)