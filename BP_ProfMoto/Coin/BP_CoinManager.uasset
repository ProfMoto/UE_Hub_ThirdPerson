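; Coin manager that keeps the coin count, handles increments and spending, and optionally triggers rewards automatically as coins accumulate.
; With AutoReward on, each increment passes the count to CoinCheck on BP_Reward actors tagged with the current AutoRewardOrder entry.
; If the order array had no valid entry at BeginPlay, it checks the first BP_Reward found instead.
; AutoRewardID++ advances to the next entry and rechecks one tick later.
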(event `AutoRewardID++`
  (`/Engine/EditorBlueprintResources/StandardMacros.IncrementInt` (`self.NextAutoReward`)
    (:`  `
      (`KismetSystemLibrary.DelayUntilNextTick`)
      (`self.ArrayCoinCheck`))))

(event `SetNextAutoReward`
  (if (not (`KismetArrayLibrary.Array_IsValidIndex` (`self.AutoRewardOrder`) (`self.NextAutoReward`)))
    (`KismetSystemLibrary.PrintString` "Auto Reward has not content")))

(event `ArrayCoinCheck`
  (bind _outactors (`GameplayStatics.GetAllActorsOfClassWithTag` "/Game/BP_ProfMoto/Coin/BP_Reward.BP_Reward_C" (`KismetStringLibrary.Conv_StringToName` (`|GetArrayItem` (`self.AutoRewardOrder`) (`self.NextAutoReward`)))))
  (bind _output_get (set `self.TaggedActors` _outactors))
  (for _array_element _output_get
    (`/Game/BP_ProfMoto/Coin/BP_Reward.CoinCheck` _array_element (`self.CoinCount`))))

(event `CoinCountIncrement`
  (`/Engine/EditorBlueprintResources/StandardMacros.IncrementInt` (`self.CoinCount`)
    (:`  `
      (if (`self.AutoReward`)
        (if (`self.ArrayContent`)
          (`self.ArrayCoinCheck`)
          (else
            (bind _returnvalue (`GameplayStatics.GetActorOfClass` "/Game/BP_ProfMoto/Coin/BP_Reward.BP_Reward_C"))
            (`/Game/BP_ProfMoto/Coin/BP_Reward.CoinCheck` _returnvalue (`self.CoinCount`))))))))

(event `ConsumeCoins`
  (params (Coins :type Integer))
  (set `self.CoinCount` (- (`self.CoinCount`) Coins)))

(event `self.ReceiveBeginPlay`
  (bind _returnvalue (`KismetArrayLibrary.Array_IsValidIndex` (`self.AutoRewardOrder`) (`self.NextAutoReward`)))
  (if (`self.AutoReward`)
    (if _returnvalue
      (set `self.ArrayContent` _returnvalue)
      (`self.SetNextAutoReward`))))

(fn `UserConstructionScript`)