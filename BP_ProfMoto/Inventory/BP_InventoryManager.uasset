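; Inventory manager actor that tallies items by integer ID in a count array.
; Its InventoryIncrement event stores the incoming ID, then increments that slot, or grows the array to fit and sets it to one when the index is invalid.
; The updated count prints on screen as debug output.
; The event is the only active logic, with no removal or lookup functions.
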(event `InventoryIncrement`
  (params (InventoryID :type Integer))
  (bind _output_get (set `self.Inventory ID` InventoryID))
  (if (`KismetArrayLibrary.Array_IsValidIndex` (`self.InventoryCountArray`) _output_get)
    (`/Engine/EditorBlueprintResources/StandardMacros.IncrementInt` (`|GetArrayItem` (`self.InventoryCountArray`) (`self.Inventory ID`))
      (:`  `
        _))
    (else
      (`KismetArrayLibrary.Array_Set` (`self.InventoryCountArray`) (`self.Inventory ID`) 1 true)))
  (`KismetSystemLibrary.PrintString` (`KismetStringLibrary.Conv_IntToString` (`|GetArrayItem` (`self.InventoryCountArray`) (`self.Inventory ID`))) true false))

(fn `UserConstructionScript`)