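; BP_HoldOneWorkbench is a workbench that checks whether enough of one inventory item is held when an actor overlaps it.
; On overlap it finds BP_HoldOneManager and compares the HoldOneArray count at InventoryID against InventoryNeeded.
; It only prints the pass or fail result and the count as debug text, without changing the inventory.
; The construction script shows the InventoryID on its text render component.
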(event `self.ReceiveBeginPlay`)

(event `self.ReceiveActorBeginOverlap`
  (params (OtherActor :type "Actor Object Reference"))
  (bind _inventoryid (`self.InventoryID`))
  (bind _returnvalue (`GameplayStatics.GetActorOfClass` "/Game/BP_ProfMoto/Inventory/BP_HoldOneManager.BP_HoldOneManager_C"))
  (if (>= (`|GetArrayItem` (`/Game/BP_ProfMoto/Inventory/BP_HoldOneManager.HoldOneArray` _returnvalue) (`self.InventoryID`)) (`self.InventoryNeeded`))
    (`KismetSystemLibrary.PrintString` "Inventory Condition Met")
    (else
      (`KismetSystemLibrary.PrintString` "Inventory Condition Failed")))
  (`KismetSystemLibrary.PrintString` (`KismetStringLibrary.Concat_StrStr` "Workbench: " (`KismetStringLibrary.Conv_IntToString` (`|GetArrayItem` (`/Game/BP_ProfMoto/Inventory/BP_HoldOneManager.HoldOneArray` _returnvalue) _inventoryid)) " of item " (`KismetStringLibrary.Conv_IntToString` _inventoryid) " out of " (`KismetStringLibrary.Conv_IntToString` (`self.InventoryNeeded`)))))

(fn `UserConstructionScript`
  (`TextRenderComponent.K2_SetText` (`self.TextRender`) (`KismetTextLibrary.Conv_IntToText` (`self.InventoryID`))))