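; BP_HoldOneIndicator is an inventory Blueprint that provides a player power-up, supersizing the character and restoring it.
; SuperSizeMe doubles the scale of CollidingPlayer and raises player 0's jump velocity and walk speed, while RestoreMe sets all three back to fixed normal values.
; Scaling targets CollidingPlayer but movement changes always target player character 0.
; Neither function is called within this Blueprint, and its event graph and construction script are empty.
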(event `self.ReceiveActorBeginOverlap`
  (params (OtherActor :type "Actor Object Reference")))

(fn `RestoreMe`
  (bind _charactermovement (`Character.CharacterMovement` (`GameplayStatics.GetPlayerCharacter` 0)))
  (`self.SetActorScale3D` (`self.collidingPlayer`) (1.0 1.0 1.0))
  (set `CharacterMovementComponent.JumpZVelocity` 700.0 _charactermovement)
  (set `CharacterMovementComponent.MaxWalkSpeed` 500.0 _charactermovement))

(fn `SuperSizeMe`
  (bind _charactermovement (`Character.CharacterMovement` (`GameplayStatics.GetPlayerCharacter` 0)))
  (`self.SetActorScale3D` (`self.collidingPlayer`) (2.0 2.0 2.0))
  (set `CharacterMovementComponent.JumpZVelocity` 1400.0 _charactermovement)
  (set `CharacterMovementComponent.MaxWalkSpeed` 1000.0 _charactermovement))

(fn `UserConstructionScript`)